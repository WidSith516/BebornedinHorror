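; Combat manager for an ATB turn-based battle system, still a work in progress.
; BeginPlay splits characters into player and enemy lists; in Fight state, Tick spawns enemies from DT_Character_Dictionary every frame.
; In Player Choose phase, the first ReadyQueue character gets a skill widget or a print-only AI stub.
; ATB accumulation would fill that queue but is never called here; QTE and skill-chosen handlers are empty.
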(event Custom|OnTurnReady%28Character%29
  (params (Ready%20Character :type BP%20Character%20Base%20Object%20Reference))
  (Utilities|Array|Add (Variables|Characterstate|GetReadyQueue) Ready%20Character))

(event Custom|OnQTEComplete%28Result%29)

(event Custom|OnSkillChosen_Event
  (params (Character :type BP%20Character%20Base%20Object%20Reference) (SkillIndex :type Integer)))

(event EventBeginPlay
  ;[1 1 1] 初始化
  (bind _outactors (Actor|GetAllActorsOfClass "/Game/BluePrint/System/Character/BP_Character_Base.BP_Character_Base_C"))
  (bind _output_get (Variables|Characterstate|SetAllCharacters _outactors))
  (for _array_element _output_get
    (bind _asbp_character_base (Utilities|Casting|CastToBP_Character_Base _array_element))
    (if (Variables|/Game/BluePrint/System/Character/BP_Character_Base.BP_Character_Base_C|GetbIsplayercontroled _asbp_character_base)
      (Utilities|Array|Add (Variables|Characterstate|GetPlayerCharacters) _asbp_character_base)
      (else
        (Utilities|Array|Add (Variables|Characterstate|GetEnemyCharacters) _asbp_character_base))))
  (Variables|Default|SetTeamAP 5)
  (Variables|Default|SetTurnCount 0)
  (Variables|Default|SetCurrentPhase "NewEnumerator4"))

(event EventTick
  (params (DeltaSeconds :type Float%20%28single-precision%29))
  (Variables|Default|SetDelta%20Seconds DeltaSeconds)
  (switch Utilities|FlowControl|Switch|SwitchonGameState (Variables|Default|GetCurrentState)
    (:NewEnumerator1
      (CallFunction|LoadBattleData (Variables|Default|GetCharacterRowID))
      (switch Utilities|FlowControl|Switch|SwitchonFPhaseEnum (Variables|Default|GetCurrentPhase)
        (:NewEnumerator1
          ;[1 1 1] 进入玩家选择阶段
          (bind _result (Math|Integer|IncrementInt (Variables|Default|GetTurnCount))
            (:%20%20
              (Development|PrintText (Utilities|Text|ToText(String) (Utilities|String|ToString(Integer) _result)))
              (if (Variables|/Game/BluePrint/System/Character/BP_Character_Base.BP_Character_Base_C|GetbIsplayercontroled (Utilities|Array|Get(acopy) (Variables|Characterstate|GetReadyQueue)))
                (CallFunction|ShowSkillSelectionUI)
                (else
                  (CallFunction|AISelectSkill))))))))))

(fn ConstructionScript)

(fn ATBAccumulation
  (for _array_element (Variables|Characterstate|GetAllCharacters)
    (bind _output_get (Variables|/Game/BluePrint/System/Character/BP_Character_Base.BP_Character_Base_C|SetATBValue _array_element (* (Variables|/Game/BluePrint/System/Character/BP_Character_Base.BP_Character_Base_C|GetATBSpeed _array_element) (Variables|Default|GetDelta%20Seconds))))
    (if (and (>= _output_get 1e+02) (Variables|/Game/BluePrint/System/Character/BP_Character_Base.BP_Character_Base_C|GetIsTurnReady _array_element))
      (Variables|/Game/BluePrint/System/Character/BP_Character_Base.BP_Character_Base_C|SetIsTurnReady _array_element true)
      (CallFunction|OnTurnReady(Character) _array_element)))
  (if (> (Utilities|Array|Length (Variables|Characterstate|GetReadyQueue)) 0)
    (Variables|Default|SetCurrentPhase "NewEnumerator1")))

(fn PlayerChoose)

(fn ShowSkillSelectionUI
  (Development|PrintString "Player is choosing Skill")
  (bind _returnvalue (UserInterface|CreateWidget "/Game/BluePrint/Widget/WBP_SkillSelection.WBP_SkillSelection_C" (Game|GetPlayerController 0)))
  (EventDispatchers|BindEventtoOnSkillChosen _returnvalue)
  (UserInterface|Viewport|AddtoViewport _returnvalue 0)
  (Default|InitializewithCharacter _returnvalue (Variables|Characterstate|GetActiveCharacter) (Variables|Default|GetTeamAP)))

(fn AISelectSkill
  (Development|PrintString "AI is Choosing Skill"))

(fn LoadBattleData
  (params (CharacterRowID :type Array%20of%20Names))
  (for _array_element CharacterRowID
    (bind _returnvalue (Utilities|GetDataTableRow "/Game/BluePrint/System/Character/DT_Character_Dictionary.DT_Character_Dictionary" _array_element)
      (:then
        (Game|SpawnActorfromClass :Class "/Game/BluePrint/System/Character/BP_EnemyCharacter.BP_EnemyCharacter_C" :CollisionHandlingOverride "Undefined" :TransformScaleMethod "MultiplyWithRoot" :Characterid (.characterid _returnvalue) :MaxHP (.maxhp _returnvalue) :ATK (.atk _returnvalue) :bIsplayercontroled (.bisplayercontroled _returnvalue) :Instigator 0))))
  (return))